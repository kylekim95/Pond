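; BP_Incident_Gorani is an incident actor that moves a gorani (deer) along a spline route.
; On BeginPlay it attaches the LeftEye component to the deer's left eye socket.
; Each Tick advances the distance along Route by walk speed, then sets the deer's local transform from the spline with a -90 degree yaw offset and the route's scale.
; When Loop is set, the distance resets to zero at the spline's end.
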(event `self.ReceiveBeginPlay`
  (`SceneComponent.K2_AttachToComponent` (`self.LeftEye`) (`self.Gorani`) "DeerDoe_LeftEye" "KeepRelative" "KeepRelative" "KeepRelative" true))

(event `self.ReceiveTick`
  (params (DeltaSeconds :type "Float (single-precision)"))
  (bind _route (`self.Route`))
  (bind _returnvalue (`SplineComponent.GetTransformAtDistanceAlongSpline` _route (`self.DistanceAlongSpline`) "Local" false))
  (set `self.DistanceAlongSpline` (+ (* DeltaSeconds (`self.GoraniWalkSpeed`)) (`self.DistanceAlongSpline`)))
  (`SceneComponent.K2_SetRelativeTransform` (`self.Gorani`) (`KismetMathLibrary.MakeTransform` (`KismetMathLibrary.MakeVector` (.x (.location _returnvalue)) (.y (.location _returnvalue)) (.z (.location _returnvalue))) (`KismetMathLibrary.MakeRotator` (.roll (.rotation _returnvalue)) (.pitch (.rotation _returnvalue)) (+ (.yaw (.rotation _returnvalue)) -90.0)) (`SceneComponent.RelativeScale3D` _route)) false false)
  (if (`self.Loop`)
    (if (>= (`self.DistanceAlongSpline`) (`SplineComponent.GetSplineLength` _route))
      (set `self.DistanceAlongSpline` 0.0))))

(fn `UserConstructionScript`)