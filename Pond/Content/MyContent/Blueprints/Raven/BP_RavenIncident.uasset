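; Raven incident actor that takes off from its spawn point, flies to a spot in the player's view and plays an eating animation.
; On BeginPlay it retries random navigable points around the player camera until one is within FOV and beyond the minimum radius.
; It builds a four-point raised path, then enqueues takeoff montage, latent movement and eating montage as actions, each setting a promise value on completion.
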(event `self.ReceiveBeginPlay`
  (bind _pathpoints (`self.PathPoints`))
  (bind _capsulecomponent (`MyPawn.CapsuleComponent` (`self.PlayerPawn`)))
  (bind (_returnvalue_x _returnvalue_y) (`KismetMathLibrary.BreakVector` (* (+ (`self.SpawnPosition`) (`self.Destination`)) (0.2 0.8 1.0))))
  (bind (_returnvalue_x_2 _returnvalue_y_2) (`KismetMathLibrary.BreakVector` (* (+ (`self.SpawnPosition`) (`self.Destination`)) (0.8 0.8 1.0))))
  (`parent.ReceiveBeginPlay`)
  (bind _asmy_pawn (cast `MyPawn` (`GameplayStatics.GetPlayerPawn` 0)))
  (set `self.PlayerPawn` _asmy_pawn)
  (set `self.SpawnPosition` (`self.K2_GetActorLocation` self))
  (bind (_randomlocation _returnvalue) (`NavigationSystemV1.K2_GetRandomLocationInNavigableRadius` (`SceneComponent.K2_GetComponentLocation` (`MyPawn.CameraComponent` (`self.PlayerPawn`))) (`self.DestinationRadiusMax`) null null :!label _label))
  (if _returnvalue
    (bind _output_get (set `self.Destination` _randomlocation))
    (bind _returnvalue_2 (`MySpawnLibrary.WithinPlayerFOV` _output_get (`SceneComponent.K2_GetComponentLocation` _capsulecomponent) (`SceneComponent.GetForwardVector` _capsulecomponent)))
    (if _returnvalue_2
      (if (> (`KismetMathLibrary.VSize` (- (`self.Destination`) (`SceneComponent.K2_GetComponentLocation` (`MyPawn.CameraComponent` (`self.PlayerPawn`))))) (`self.DestinationRadiusMin`))
        (`|ExecutionSequence`
          (:`then_0`
            (`KismetArrayLibrary.Array_Add` _pathpoints (`self.SpawnPosition`))
            (`KismetArrayLibrary.Array_Add` _pathpoints (`KismetMathLibrary.MakeVector` _returnvalue_x _returnvalue_y 500.0))
            (`KismetArrayLibrary.Array_Add` _pathpoints (`KismetMathLibrary.MakeVector` _returnvalue_x_2 _returnvalue_y_2 1000.0))
            (`KismetArrayLibrary.Array_Add` _pathpoints (`self.Destination`)))
          (:`then_1`
            (`self.EnqueueAction` (delegate `PlayMontage`)))
          (:`then_2`
            (`self.EnqueueAction` (delegate `MoveTo`)))
          (:`then_3`
            (`self.EnqueueAction` (delegate `PlayMontage2`))))
        (else
          (goto _label)))
      (else
        (goto _label)))
    (else
      (goto _label))))

(event `PlayMontage`
  (params (Params :type String))
  (`|PlayMontage` (`self.SkeletalMesh`) "/Game/MyContent/Blueprints/Raven/AM_RavenTakeOff.AM_RavenTakeOff"
    (:`OnCompleted`
      (`self.SetPromiseValue` "REGULAR"))))

(event `MoveTo`
  (params (Params :type String))
  (bind _asbp_raven_incident (cast `/Game/MyContent/Blueprints/Raven/BP_RavenIncident` self))
  (`MyAsyncActions.LatentActorMovement` (`self.PathPoints`) _asbp_raven_incident (`self.Grounded`)
    (:`OnCompleted`
      (`self.SetPromiseValue` "REGULAR"))))

(event `PlayMontage2`
  (params (Params :type String))
  (`|PlayMontage` (`self.SkeletalMesh`) "/Game/MyContent/Blueprints/Raven/AM_RavenEatSomething.AM_RavenEatSomething"
    (:`OnCompleted`
      (`self.SetPromiseValue` "REGULAR"))))

(fn `UserConstructionScript`)