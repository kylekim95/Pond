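; Incident actor for a gorani (deer) that walks from its spawn point to a spot in the player's view, then grazes.
; BeginPlay retries random navmesh points until one lies within the player's FOV beyond a minimum distance, then line-traces path points onto surfaces.
; Move and graze run as queued actions that each set a promise value when done.
; Tick copies the latent movement's velocity, and debug drawing shows the path and boundary planes.
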(event `self.ReceiveBeginPlay`
  (bind _capsulecomponent (`MyPawn.CapsuleComponent` (`self.PlayerPawn`)))
  (`parent.ReceiveBeginPlay`)
  (bind _asmy_pawn (cast `MyPawn` (`GameplayStatics.GetPlayerPawn` 0)))
  (set `self.PlayerPawn` _asmy_pawn)
  (set `self.SpawnPosition` (`self.K2_GetActorLocation` self))
  ;[1 1 1] Init Destination
  (bind (_randomlocation _returnvalue) (`NavigationSystemV1.K2_GetRandomLocationInNavigableRadius` (`SceneComponent.K2_GetComponentLocation` (`MyPawn.CameraComponent` (`self.PlayerPawn`))) (`self.DestinationRadiusMax`) null null :!label _label))
  (if _returnvalue
    (bind _output_get (set `self.Destination` _randomlocation))
    (bind _returnvalue_2 (`MySpawnLibrary.WithinPlayerFOV` _output_get (`SceneComponent.K2_GetComponentLocation` _capsulecomponent) (`SceneComponent.GetForwardVector` _capsulecomponent)))
    (if _returnvalue_2
      (if (> (`KismetMathLibrary.VSize` (- (`self.Destination`) (`SceneComponent.K2_GetComponentLocation` (`MyPawn.CameraComponent` (`self.PlayerPawn`))))) (`self.DestinationRadiusMin`))
        (`|ExecutionSequence`
          (:`then_0`
            (bind _returnvalue_3 (`NavigationSystemV1.FindPathToLocationSynchronously` (`self.SpawnPosition`) (`self.Destination`) null null))
            (bind _output_get_2 (set `self.Path` (`NavigationPath.PathPoints` _returnvalue_3)))
            (for (_array_element _array_index) _output_get_2
              (bind (_outhit _returnvalue_4) (`KismetSystemLibrary.LineTraceSingle` _array_element (+ _array_element (`KismetMathLibrary.MakeVector` 0.0 0.0 (* (.z _array_element) -2.0))) "TraceTypeQuery1"))
              (if _returnvalue_4
                (`KismetArrayLibrary.Array_Set` (`self.Path`) _array_index (`.Location` (`GameplayStatics.BreakHitResult` _outhit)))
                (`KismetSystemLibrary.DrawDebugLine` _array_element (+ _array_element (0.0 0.0 250.0)) (struct :`R` 1.0 :`A` 1.0) 1000.0 2.0))))
          (:`then_1`
            (`self.EnqueueAction` (delegate `MoveToDest`)))
          (:`then_2`
            (`self.EnqueueAction` (delegate `GrazeOnce`))))
        (else
          (goto _label)))
      (else
        (goto _label)))
    (else
      (goto _label))))

(event `MoveToDest`
  (params (Params :type String))
  (bind _asbp_gorani_incident (cast `/Game/MyContent/Blueprints/BP_GoraniIncident` self))
  (bind (_boundarynormals _pointsonboundary _currentvelocity) (`MyAsyncActions.LatentActorMovement` (`self.Path`) _asbp_gorani_incident)
    (:`OnStarted`
      (for _index (range (`KismetArrayLibrary.Array_Length` _boundarynormals))
        (bind _output (`|GetArrayItem` _pointsonboundary _index))
        (`KismetSystemLibrary.DrawDebugPlane` (`KismetMathLibrary.MakePlaneFromPointAndNormal` _output (`|GetArrayItem` _boundarynormals _index)) (+ _output (0.0 0.0 60.0)) 50.0 (struct :`R` 1.0 :`B` 1.0 :`A` 0.25) 1000.0)))
    (:`OnCancelled`
      (`self.SetPromiseValue` "REGULAR" :!label _label_2)
      (`KismetSystemLibrary.PrintString` "DONE"))
    (:`OnCompleted`
      (goto _label_2))))

(event `self.ReceiveTick`
  (params (DeltaSeconds :type "Float (single-precision)"))
  (`parent.ReceiveTick` DeltaSeconds)
  (set `self.Velocity` (stale `MoveToDest` _currentvelocity)))

(event `GrazeOnce`
  (params (Params :type String))
  (`|PlayMontage` (`self.SKM_Gorani`) "/Game/MyContent/Blueprints/AnimMontage_DeerDoe_GrazeOnce.AnimMontage_DeerDoe_GrazeOnce"
    (:`OnCompleted`
      (`self.SetPromiseValue` "REGULAR"))))

(fn `LightPillar`
  (params (Position :type "Vector Structure") (Color :type "LinearColor Structure"))
  (`KismetSystemLibrary.DrawDebugLine` Position (+ Position (0.0 0.0 200.0)) Color 1000.0 3.0))

(fn `UserConstructionScript`)